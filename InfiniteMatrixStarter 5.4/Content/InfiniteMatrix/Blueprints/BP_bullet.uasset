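; BP_bullet is a player projectile that destroys enemies and awards score.
; RegisterPlayerRef stores the player and sets the bullet's speed to the player's forward speed plus a fixed boost.
; Tick moves it along world X and destroys it once it gets a set distance ahead of the controlled player pawn.
; Overlapping a BP_enemy child destroys both actors, increments the player's score and updates the health widget's score display.
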(event `self.ReceiveActorBeginOverlap`
  (params (OtherActor :type "Actor Object Reference"))
  (bind _playerref (`self.playerRef`))
  (if (`KismetMathLibrary.ClassIsChildOf` (`GameplayStatics.GetObjectClass` OtherActor) "/Game/InfiniteMatrix/Blueprints/BP_enemy.BP_enemy_C")
    (`self.K2_DestroyActor` OtherActor)
    (`self.K2_DestroyActor`)
    (bind _output_get (set `/Game/InfiniteMatrix/Blueprints/BP_Player.scorePlayer` (+ (`/Game/InfiniteMatrix/Blueprints/BP_Player.scorePlayer` _playerref) 1) _playerref))
    (`/Game/InfiniteMatrix/UI/WBP_health.updateScore` (`/Game/InfiniteMatrix/Blueprints/BP_Player.healthWidget` _playerref) _output_get)))

(event `self.ReceiveTick`
  (params (DeltaSeconds :type "Float (single-precision)"))
  (bind _returnvalue_x (`KismetMathLibrary.BreakVector` (`self.K2_GetActorLocation`)))
  (`self.K2_AddActorWorldOffset` (`KismetMathLibrary.MakeVector` (* DeltaSeconds (`self.forwardSpeed`))))
  (bind _asbp_player (cast `/Game/InfiniteMatrix/Blueprints/BP_Player` (`Controller.K2_GetPawn` (`GameplayStatics.GetPlayerController` 0))))
  (bind _returnvalue_x_2 (`KismetMathLibrary.BreakVector` (`self.K2_GetActorLocation` _asbp_player)))
  (if (>= (- _returnvalue_x _returnvalue_x_2) 1000.0)
    (`self.K2_DestroyActor`)))

(fn `registerPlayerRef`
  (params (playerRefParam :type "/Game/InfiniteMatrix/Blueprints/BP_Player Object Reference"))
  (bind _output_get (set `self.playerRef` playerRefParam))
  (set `self.forwardSpeed` (`KismetMathLibrary.FTrunc` (+ (`/Game/InfiniteMatrix/Blueprints/BP_Player.forwardSpeed` _output_get) 1000.0))))

(fn `UserConstructionScript`)