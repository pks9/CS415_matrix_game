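; BP_Tunnel is a tunnel segment with a rotating obstacle wall that can also be a health pack.
; Passing its trigger adds score, asks TunnelSpawner for another segment, then destroys this one and its enemy.
; Touching the wall damages the player or, for a pack, heals within 100, deducting a point whenever health is updated.
; RandomizeWall picks mesh and roll through chained checks that each reroll, so sometimes none is set.
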(event `self.ReceiveTick`
  (params (DeltaSeconds :type "Float (single-precision)"))
  (`SceneComponent.K2_AddLocalRotation` (`self.wallMesh`) (`KismetMathLibrary.MakeRotator` (* DeltaSeconds (`self.rotateSpeed`))) false false))

(event `self.triggerZone.OnComponentBeginOverlap`
  (params (OverlappedComponent :type "PrimitiveComponent Object Reference") (OtherActor :type "Actor Object Reference") (OtherComp :type "PrimitiveComponent Object Reference") (OtherBodyIndex :type Integer) (bFromSweep :type Boolean) (SweepResult :type "HitResult Structure (by ref)"))
  (bind _enemyref (`self.enemyRef`))
  (bind _asbp_player (cast `/Game/InfiniteMatrix/Blueprints/BP_Player` OtherActor))
  (bind _output_get (set `/Game/InfiniteMatrix/Blueprints/BP_Player.scorePlayer` (+ (`/Game/InfiniteMatrix/Blueprints/BP_Player.scorePlayer` _asbp_player) 1) _asbp_player))
  (`/Game/InfiniteMatrix/UI/WBP_health.updateScore` (`/Game/InfiniteMatrix/Blueprints/BP_Player.healthWidget` _asbp_player) _output_get)
  (`/Game/InfiniteMatrix/Blueprints/BP_TunnelSpawner.spawnTunnelAtPoint` (`self.tunnelSpawner`))
  (if (`KismetSystemLibrary.IsValid` _enemyref)
    (`self.K2_DestroyActor` _enemyref))
  (`self.K2_DestroyActor`))

(event `self.wallMesh.OnComponentBeginOverlap`
  (params (OverlappedComponent :type "PrimitiveComponent Object Reference") (OtherActor :type "Actor Object Reference") (OtherComp :type "PrimitiveComponent Object Reference") (OtherBodyIndex :type Integer) (bFromSweep :type Boolean) (SweepResult :type "HitResult Structure (by ref)"))
  (bind _asbp_player (cast `/Game/InfiniteMatrix/Blueprints/BP_Player` OtherActor))
  (if (== (`StaticMeshComponent.StaticMesh` (`self.wallMesh`)) "/Game/InfiniteMatrix/Meshes/SM_health_pack.SM_health_pack")
    (bind _health (`/Game/InfiniteMatrix/Blueprints/BP_Player.health` _asbp_player))
    (bind _returnvalue (+ _health 10))
    (if (<= _returnvalue 100)
      (set `self.newHealth` _returnvalue)
      (bind _output_get (set `/Game/InfiniteMatrix/Blueprints/BP_Player.health` (`self.newHealth`) _asbp_player :!label _label))
      (bind _healthwidget (`/Game/InfiniteMatrix/Blueprints/BP_Player.healthWidget` _asbp_player))
      (`/Game/InfiniteMatrix/UI/WBP_health.updateHealth` _healthwidget _output_get)
      (if (<= _output_get 0)
        (`/Game/InfiniteMatrix/Blueprints/BP_Player.displayRestart` _asbp_player))
      (bind _output_get_2 (set `/Game/InfiniteMatrix/Blueprints/BP_Player.scorePlayer` (- (`/Game/InfiniteMatrix/Blueprints/BP_Player.scorePlayer` _asbp_player) 1) _asbp_player))
      (`/Game/InfiniteMatrix/UI/WBP_health.updateScore` _healthwidget _output_get_2))
    (else
      (set `self.newHealth` (- _health 10))
      (goto _label))))

(fn `randomizeWall`
  (bind _returnvalue (`KismetMathLibrary.RandomIntegerInRange` 0 100))
  (if (< _returnvalue 10)
    (set `self.randInd` 4)
    (`StaticMeshComponent.SetStaticMesh` (`self.wallMesh`) (select `int` (`self.randInd`) :`0` "/Game/InfiniteMatrix/Meshes/SM_Hole_01.SM_Hole_01" :`1` "/Game/InfiniteMatrix/Meshes/SM_Hole_02.SM_Hole_02" :`2` "/Game/InfiniteMatrix/Meshes/SM_Hole_03.SM_Hole_03" :`3` "/Game/InfiniteMatrix/Meshes/SM_Hole_04.SM_Hole_04" :`4` "/Game/InfiniteMatrix/Meshes/SM_health_pack.SM_health_pack" :!type "StaticMesh Object Reference") :!label _label)
    (`SceneComponent.K2_AddLocalRotation` (`self.wallMesh`) (`KismetMathLibrary.MakeRotator` (`KismetMathLibrary.RandomFloatInRange` 0.0 360.0)) false false)
    (elif (`KismetMathLibrary.InRange_IntInt` _returnvalue 10 32)
      (set `self.randInd` 2)
      (goto _label)
      (elif (`KismetMathLibrary.InRange_IntInt` _returnvalue 33 54)
        (set `self.randInd` 1)
        (goto _label)
        (elif (`KismetMathLibrary.InRange_IntInt` _returnvalue 55 76)
          (set `self.randInd` 0)
          (goto _label)
          (elif (`KismetMathLibrary.InRange_IntInt` _returnvalue 77 100)
            (set `self.randInd` 3)
            (goto _label)))))))

(fn `UserConstructionScript`)